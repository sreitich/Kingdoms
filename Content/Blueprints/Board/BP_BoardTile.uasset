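; BP_BoardTile is a board tile with an emissive highlight light that can be revealed or hidden.
; UpdateEmissiveHighlight sets the light's color and visibility, then plays or reverses HighlightTimeline at the supplied rate.
; The timeline's Delta track feeds an FInterpTo toward TileLightBrightness to drive light intensity.
; Visibility switches off immediately on hide, before the timeline reverses.
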(event `self.UpdateEmissiveHighlight`
  (params (bReveal :type Boolean) (PlayRate :type "Float (single-precision)") (Color :type "LinearColor Structure"))
  ;[1 1 1] Update and reveal/hide this tile's emissive highlight.
  (`LightComponent.SetLightColor` (`self.EmissiveHighlight`) Color true)
  (`SceneComponent.SetVisibility` (`self.EmissiveHighlight`) bReveal false)
  (`TimelineComponent.SetPlayRate` (`self.Highlight Timeline`) PlayRate)
  (if bReveal
    (bind (_direction _delta) (`Timeline|Highlight Timeline` :!label _label)
      (:`Update`
        (`LightComponent.SetIntensity` (`self.EmissiveHighlight`) (`KismetMathLibrary.FInterpTo` 0.0 (`self.TileLightBrightness`) _delta 1.0))))
    (else
      (goto _label :!via `Reverse`))))

(fn `UserConstructionScript`)