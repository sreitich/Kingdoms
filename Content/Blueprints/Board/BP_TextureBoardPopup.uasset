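; Board popup actor that shows a given texture on a billboard and animates it into view.
; ActivatePopup sets the sprite, then plays a timeline whose Height and Scale tracks drive a rise from below the actor's placed location and growth from a fraction of its size.
; Each update toggles the billboard's visibility off and on to force its scale to refresh.
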(event `self.ActivatePopup`
  (params (Texture :type "Texture2D Object Reference"))
  (bind _displayedtexture (`self.DisplayedTexture`))
  (`BillboardComponent.SetSprite` (`self.DisplayedTexture`) Texture)
  (set `self.StartingLocation` (- (`self.K2_GetActorLocation`) (0.0 0.0 50.0)))
  (set `self.StartingScale` (/ (`SceneComponent.RelativeScale3D` (`self.DisplayedTexture`)) 5.0))
  (bind (_direction _height _scale) (`Timeline|Popup Animation`)
    (:`Update`
      ;[1 1 1] Start 50 units below the desired location and interpolate upward
      (`self.K2_SetActorLocation` (+ (* (0.0 0.0 50.0) (`KismetMathLibrary.Conv_DoubleToVector` _height)) (`self.StartingLocation`)))
      ;[1 1 1] Start at 1/5th the desired scale and interpolate up
      (`SceneComponent.SetWorldScale3D` (`self.DisplayedTexture`) (* (`self.StartingScale`) (* _scale 5.0)))
      ;[1 1 1] Billboard scale updates don't refresh automatically. This is a little cheat for that.
      (`SceneComponent.SetVisibility` _displayedtexture false false)
      (`SceneComponent.SetVisibility` _displayedtexture true false))))

(fn `UserConstructionScript`)