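; A world-space board pop-up actor that shows a modifier's value change and strength through a widget turned toward the local player's camera each tick.
; On activation a timeline animates its height and scale, then a timer holds it for the given duration before reversing the animation.
; It can follow its base actor's PopUpLocationComponent.
; After reversing it calls OnModifierPopUpFinished for the next queued pop-up and destroys itself.
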(event `self.BP_ActivateModifierPopUp`
  (params (BaseActor :type "Actor Object Reference") (Location :type "Vector Structure") (ValueChange :type Integer) (bStrength :type Boolean) (Duration :type "Float (single-precision)") (bFollowActor :type Boolean))
  (set `self.Base Actor` BaseActor)
  (set `self.Follow Actor` bFollowActor)
  (set `self.Spawn Location` Location)
  (bind _aswbp_match_modifier_board_pop_up_widget (cast `/Game/Blueprints/UserInterface/Match/WBP_Match_ModifierBoardPopUpWidget` (`WidgetComponent.GetUserWidgetObject` (`self.Widget`))))
  (`Match_ModifierBoardPopUpWidget.UpdateModifierWidget` _aswbp_match_modifier_board_pop_up_widget ValueChange bStrength) ; Update the pop-up widget's displayed information.
  (`SceneComponent.SetHiddenInGame` (`self.Widget`) false false) ; Reveal the pop-up widget.
  (set `self.Interpolating` true)
  (bind (_direction _delta_height _delta_scale) (`Timeline|New Pop-Up Timeline` :!label _label)
    (:`Update`
      (`self.K2_SetActorLocation` (`KismetMathLibrary.MakeVector` (.x (`self.Spawn Location`)) (.y (`self.Spawn Location`)) (* (.z (`self.Spawn Location`)) _delta_height))) ; Animate this pop-up's height.
      (`self.SetActorRelativeScale3D` (`KismetMathLibrary.MakeVector` _delta_scale _delta_scale _delta_scale)) ; Animate this pop-up's scale.
    )
    (:`Finished`
      (set `self.Interpolating` false)
      (switch `ETimelineDirection` _direction
        (:`Forward`
          (`KismetSystemLibrary.K2_SetTimerDelegate` (delegate `Destoy Pop-Up`) Duration) ; Wait for the given duration before destroying the pop-up
        )
        (:`Backward`
          (`self.OnModifierPopUpFinished`) ; Play the next queued pop-up.
          (`self.K2_DestroyActor`) ; Destroy the pop-up after reversing its animation.
        )))))

(event `Destoy Pop-Up`
  (set `self.Interpolating` true)
  (goto _label :!via `Reverse`))

(event `self.ReceiveTick`
  (params (DeltaSeconds :type "Float (single-precision)"))
  (bind _widget (`self.Widget`))
  ;[1 1 1] Rotate the pop-up to face the local player every tick.
  (bind _asbp_match_player_pawn (cast `/Game/Blueprints/Framework/Match/BP_Match_PlayerPawn` (`GameplayStatics.GetPlayerPawn` 0)))
  (`SceneComponent.K2_SetWorldRotation` _widget (`KismetMathLibrary.FindLookAtRotation` (`SceneComponent.K2_GetComponentLocation` _widget) (`SceneComponent.K2_GetComponentLocation` (`Match_PlayerPawn.Camera` _asbp_match_player_pawn))) false false)
  ;[1 1 1] Set the pop-up's location to stay at the base actor's pop-up location.
  (if (`self.Follow Actor`)
    (bind _output_get (set `self.Spawn Location` (`SceneComponent.K2_GetComponentLocation` (`self.GetComponentByClass` (`self.Base Actor`) "/Script/Kingdoms.PopUpLocationComponent")))) ; Update the pop-up's base location\nto its target actor's current location.
    (if (not (`self.Interpolating`))
      (`self.K2_SetActorLocation` _output_get) ; Manually update the pop-up's location if the timeline isn't.
    )))

(fn `UserConstructionScript`)