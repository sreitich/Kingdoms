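; BP_ParentPiece is a base Blueprint for pieces, providing a timed highlight flash on a piece's material.
; FlashHighlightTimeline fades the dynamic material's FresnelColor and Brightness to new values, holds for a duration, then fades back through a second timeline.
; The caller supplies both original and highlight values, and the Speed input scales only the fade-in's play rate.
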(event `self.FlashHighlightTimeline`
  (params (NewColor :type "LinearColor Structure") (NewBrightness :type "Float (single-precision)") (OriginalColor :type "LinearColor Structure") (OriginalBrightness :type "Float (single-precision)") (Speed :type "Float (single-precision)") (Duration :type "Float (single-precision)"))
  (bind _dynamicmaterial (`self.DynamicMaterial`))
  (bind _dynamicmaterial_2 (`self.DynamicMaterial`))
  ;[1 1 1 1 14] Set the speed of the fade
  (`TimelineComponent.SetPlayRate` (`self.Fade Into Highlight Timeline`) Speed)
  ;[1 1 1 1 14] Fade into the highlight
  (bind (_direction _alpha) (`Timeline|Fade Into Highlight Timeline` :!via `PlayFromStart`)
    (:`Update`
      (`MaterialInstanceDynamic.SetVectorParameterValue` _dynamicmaterial_2 "FresnelColor" (`KismetMathLibrary.LinearColorLerp` OriginalColor NewColor _alpha))
      (`MaterialInstanceDynamic.SetScalarParameterValue` _dynamicmaterial_2 "Brightness" (`KismetMathLibrary.Lerp` OriginalBrightness NewBrightness _alpha)))
    (:`Finished`
      ;[1 1 1 1 14] Wait with the highlight
      (`KismetSystemLibrary.Delay` Duration)
      ;[1 1 1 1 14] Fade out of the highlight
      (bind (_direction_2 _alpha_2) (`Timeline|Fade Out of Highlight Timeline` :!via `PlayFromStart`)
        (:`Update`
          (`MaterialInstanceDynamic.SetVectorParameterValue` _dynamicmaterial "FresnelColor" (`KismetMathLibrary.LinearColorLerp` NewColor OriginalColor _alpha_2))
          (`MaterialInstanceDynamic.SetScalarParameterValue` _dynamicmaterial "Brightness" (`KismetMathLibrary.Lerp` NewBrightness OriginalBrightness _alpha_2)))))))

(fn `UserConstructionScript`)