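; BP_Assassin is a rogue game piece whose active ability, Backstab, buffs its strength for an attack on a chosen target.
; The ability adds a one-duration modifier through the player pawn's networking component, stores the attack in the game state, disables every player's input, then calls ServerAttack with camera movement.
; The construction script binds modular body meshes to the main mesh's pose and attaches the pop-up component to the head.
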(event `self.BP_OnActiveAbility`
  (params (Target :type "ParentPiece Object Reference"))
  ;[1 1 1] Give the Assassin its "Backstab" modifier for this attack.
  (bind _returnvalue (`|GetDataTableRow` (`self.PieceDataTable`) (`self.PieceID`))
    (:`then`
      (bind _asbp_match_player_pawn (cast `/Game/Blueprints/Framework/Match/BP_Match_PlayerPawn` (`self.GetInstigator`)))
      (bind (_piecename _classtype _rarity _basearmor _basestrength _piecedes _classref _piececardportrait _pieceinfophoto _attackpreviewphoto _activename) (break `PieceDataStruct` _returnvalue))
      (`PieceNetworkingComponent.Server_AddModifier` (`Match_PlayerPawn.PieceNetworkingComponent` _asbp_match_player_pawn) self (make `Modifier` self "E_Friendly" _piecename _activename 1 (`self.StrengthBuffValue`) 0 false 1 false) true)
      ;[1 1 1] Save the target in the game state to be used later when starting the attack.
      (bind _asbp_match_game_state_base (cast `/Game/Blueprints/Framework/Match/BP_Match_GameStateBase` (`GameplayStatics.GetGameState`)))
      (set `Match_GameStateBase.CurrentAttackInfo` (make `AttackInfo` self Target) _asbp_match_game_state_base)
      ;[1 1 1] Disable each client's input.
      (bind _asbp_match_player_pawn_2 (`/Game/Blueprints/Libraries/ActorMacroLibrary.Execute For Each Player's Pawn`)
        (:`Completed`
          ;[1 1 1] Start the attack.
          (bind _asbp_match_game_state_base_2 (cast `/Game/Blueprints/Framework/Match/BP_Match_GameStateBase` (`GameplayStatics.GetGameState`)))
          (bind _asmatch_player_pawn (cast `Match_PlayerPawn` (`self.GetInstigator`)))
          (`Match_PlayerPawn.Server_Attack` _asmatch_player_pawn (`Match_GameStateBase.CurrentAttackInfo` _asbp_match_game_state_base_2) true)
          (`self.OnActiveAbilityEnded`) ; End this piece's active ability.
        )
        (:`For Each Pawn...`
          (`/Game/Blueprints/Framework/Match/BP_Match_PlayerPawn.Client_DisablePlayerInput` _asbp_match_player_pawn_2 true))))))

(fn `UserConstructionScript`
  (`SkinnedMeshComponent.SetLeaderPoseComponent` (`self.Head`) (`self.Mesh`) false)
  (`SkinnedMeshComponent.SetLeaderPoseComponent` (`self.Torso`) (`self.Mesh`) false)
  (`SkinnedMeshComponent.SetLeaderPoseComponent` (`self.Eyebrows`) (`self.Mesh`) false)
  (`SkinnedMeshComponent.SetLeaderPoseComponent` (`self.Left Shoulder Attachment`) (`self.Mesh`) false)
  (`SkinnedMeshComponent.SetLeaderPoseComponent` (`self.Upper Right Arm`) (`self.Mesh`) false)
  (`SkinnedMeshComponent.SetLeaderPoseComponent` (`self.Upper Left Arm`) (`self.Mesh`) false)
  (`SkinnedMeshComponent.SetLeaderPoseComponent` (`self.Lower Right Arm`) (`self.Mesh`) false)
  (`SkinnedMeshComponent.SetLeaderPoseComponent` (`self.Lower Left Arm`) (`self.Mesh`) false)
  (`SkinnedMeshComponent.SetLeaderPoseComponent` (`self.Right Hand`) (`self.Mesh`) false)
  (`SkinnedMeshComponent.SetLeaderPoseComponent` (`self.Hips`) (`self.Mesh`) false)
  (`SkinnedMeshComponent.SetLeaderPoseComponent` (`self.Left Hand`) (`self.Mesh`) false)
  (`SkinnedMeshComponent.SetLeaderPoseComponent` (`self.Left Leg`) (`self.Mesh`) false)
  (`SkinnedMeshComponent.SetLeaderPoseComponent` (`self.Hip Attachment`) (`self.Mesh`) false)
  (`SkinnedMeshComponent.SetLeaderPoseComponent` (`self.Right Leg`) (`self.Mesh`) false)
  (`SkinnedMeshComponent.SetLeaderPoseComponent` (`self.Hood`) (`self.Mesh`) false)
  (`SkinnedMeshComponent.SetLeaderPoseComponent` (`self.Hip Attachment 2`) (`self.Mesh`) false)
  (set `self.DamagedParticleAttachment` (`self.Torso`))
  (`SceneComponent.K2_AttachToComponent` (`self.PopUpLocationComponent`) (`self.Head`) "None" "KeepWorld" "KeepWorld" "KeepWorld" true))