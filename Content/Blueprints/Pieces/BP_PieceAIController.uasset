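; AI controller for board pieces that moves its piece between tiles and animates highlight flashes.
; On authority, it runs AIMoveTo to a point above the tile, then fires the piece's completion hook and optionally returns the instigating player to piece selection.
; Highlights use two timelines to blend fresnel color and brightness on the piece's dynamic material, fading back out unless indefinite.
; A disconnected rotation-reset chain never runs.
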(event `self.MovePieceToTile`
  (params (NewTile :type "BoardTile Object Reference") (bResetStateWhenFinished :type Boolean))
  (bind (_returnvalue_x _returnvalue_y _returnvalue_z) (`KismetMathLibrary.BreakVector` (`self.K2_GetActorLocation` NewTile)))
  ;[1 1 1] Moves a piece to a given tile.
  (if (and (`KismetSystemLibrary.IsValid` NewTile) (`self.HasAuthority`))
    (`AITask_MoveTo.AIMoveTo` self (`KismetMathLibrary.MakeVector` _returnvalue_x _returnvalue_y (+ _returnvalue_z 165.0)) null -1.0 "Disable" "Disable"
      (:`OnMoveFinished`
        ;[1 1 1] Call any piece-specific logic that needs to execute when a piece finishes moving to a new tile.
        (bind _asparent_piece (cast `ParentPiece` (`self.K2_GetPawn`)))
        (`ParentPiece.OnMoveToTileCompleted` _asparent_piece)
        ;[1 1 1] Reset the player's state when finished if requested.
        (if bResetStateWhenFinished
          (bind _asmatch_player_pawn (cast `Match_PlayerPawn` (`self.GetInstigator` (`self.K2_GetPawn`))))
          (bind _asbp_match_player_state (cast `/Game/Blueprints/Framework/Match/BP_Match_PlayerState` (`Pawn.PlayerState` _asmatch_player_pawn)))
          (`Match_PlayerState.Server_SetPlayerStatus` _asbp_match_player_state "E_SelectingPiece"))))))

(event `self.FlashHighlightTimeline`
  (params (PieceToHighlight :type "ParentPiece Object Reference") (NewColor :type "LinearColor Structure") (NewBrightness :type "Float (single-precision)") (OriginalColor :type "LinearColor Structure") (OriginalBrightness :type "Float (single-precision)") (PlayRate :type "Float (single-precision)") (Duration :type "Float (single-precision)") (bIndefiniteDuration :type Boolean))
  (bind _returnvalue (`ParentPiece.GetDynamicMaterial` PieceToHighlight))
  ;[1 1 1] Flashes a highlight over this controller's piece for a given duration.
  ;;[1 1 1 1 14] Set the speed of the fade
  (`TimelineComponent.SetPlayRate` (`self.Fade Into Highlight Timeline`) PlayRate)
  (`TimelineComponent.SetPlayRate` (`self.Fade Out of Highlight Timeline`) PlayRate)
  ;;[1 1 1 1 14] Fade into the highlight
  (bind (_direction _alpha) (`Timeline|Fade Into Highlight Timeline` :!via `PlayFromStart`)
    (:`Update`
      (`/Engine/EditorBlueprintResources/StandardMacros.IsValid` PieceToHighlight
        (:`Is Valid`
          (`MaterialInstanceDynamic.SetVectorParameterValue` _returnvalue "FresnelColor" (`KismetMathLibrary.LinearColorLerp` OriginalColor NewColor _alpha))
          (`MaterialInstanceDynamic.SetScalarParameterValue` _returnvalue "Brightness" (`KismetMathLibrary.Lerp` OriginalBrightness NewBrightness _alpha)))))
    (:`Finished`
      (if (not bIndefiniteDuration)
        ;;[1 1 1 1 14] Wait with the highlight
        (`KismetSystemLibrary.Delay` Duration)
        ;;[1 1 1 1 14] Fade out of the highlight
        (bind (_direction_2 _alpha_2) (`Timeline|Fade Out of Highlight Timeline` :!via `PlayFromStart`)
          (:`Update`
            (`MaterialInstanceDynamic.SetVectorParameterValue` _returnvalue "FresnelColor" (`KismetMathLibrary.LinearColorLerp` NewColor OriginalColor _alpha_2))
            (`MaterialInstanceDynamic.SetScalarParameterValue` _returnvalue "Brightness" (`KismetMathLibrary.Lerp` NewBrightness OriginalBrightness _alpha_2))))))))

(fn `UserConstructionScript`)