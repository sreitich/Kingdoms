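; Guardian piece Blueprint for the Paladins, with a targeted active ability tied to a shield effect.
; On activation it stores the target and its own rotation, turns toward the target, then multicasts a flag to its AnimBP to play the animation.
; When the effect ends, it destroys actors attached to the target that it owns.
; Construction slaves modular body meshes to the main mesh's pose and attaches the pop-up location to the head.
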(event `self.BP_OnActiveAbility`
  (params (Target :type "ParentPiece Object Reference"))
  ;[1 1 1] Active ability script.
  (set `self.ActiveAbilityTarget` Target) ; Set the target on the server.
  (bind _output_get (set `self.RotBeforeAbility` (`self.K2_GetActorRotation`))) ; Save the rotation to return to\nafter using the ability.
  (`self.InterpolatePieceRotation` null _output_get (`KismetMathLibrary.FindLookAtRotation` (`self.K2_GetActorLocation`) (`self.K2_GetActorLocation` (`self.ActiveAbilityTarget`)))) ; Face the Guardian towards its target.
  (`self.Multicast_AnimateActiveAbility`) ; Animate the active ability.
)

(event `Multicast_AnimateActiveAbility`
  ;[1 1 1] Trigger the active ability animation.
  (bind _asguardian_anim_bp (cast `/Game/Animations/Paladins/Guardian/Guardian_AnimBP` (`SkeletalMeshComponent.GetAnimInstance` (`self.Mesh`))))
  (set `AnimInstance_Parent.bUsingActive` true _asguardian_anim_bp))

(event `self.BP_OnAbilityEffectEnded`
  ;[1 1 1] Get the target piece's shield actor.
  (for _array_element (`self.GetAttachedActors` (`self.ActiveAbilityTarget`) true)
    (if (== (`self.GetOwner` _array_element) self)
      ;[1 1 1] Destroy the shield effect.
      (`self.K2_DestroyActor` _array_element))))

(fn `UserConstructionScript`
  (`SkinnedMeshComponent.SetLeaderPoseComponent` (`self.Head`) (`self.Mesh`) false)
  (`SkinnedMeshComponent.SetLeaderPoseComponent` (`self.Eyebrows`) (`self.Mesh`) false)
  (`SkinnedMeshComponent.SetLeaderPoseComponent` (`self.Hair`) (`self.Mesh`) false)
  (`SkinnedMeshComponent.SetLeaderPoseComponent` (`self.Facial Hair`) (`self.Mesh`) false)
  (`SkinnedMeshComponent.SetLeaderPoseComponent` (`self.Torso`) (`self.Mesh`) false)
  (`SkinnedMeshComponent.SetLeaderPoseComponent` (`self.Right Shoulder Attachment`) (`self.Mesh`) false)
  (`SkinnedMeshComponent.SetLeaderPoseComponent` (`self.Upper Right Arm`) (`self.Mesh`) false)
  (`SkinnedMeshComponent.SetLeaderPoseComponent` (`self.Upper Left Arm`) (`self.Mesh`) false)
  (`SkinnedMeshComponent.SetLeaderPoseComponent` (`self.Lower Right Arm`) (`self.Mesh`) false)
  (`SkinnedMeshComponent.SetLeaderPoseComponent` (`self.Lower Left Arm`) (`self.Mesh`) false)
  (`SkinnedMeshComponent.SetLeaderPoseComponent` (`self.Right Hand`) (`self.Mesh`) false)
  (`SkinnedMeshComponent.SetLeaderPoseComponent` (`self.Left Hand`) (`self.Mesh`) false)
  (`SkinnedMeshComponent.SetLeaderPoseComponent` (`self.Hips`) (`self.Mesh`) false)
  (`SkinnedMeshComponent.SetLeaderPoseComponent` (`self.Right Leg`) (`self.Mesh`) false)
  (`SkinnedMeshComponent.SetLeaderPoseComponent` (`self.Left Leg`) (`self.Mesh`) false)
  (`SkinnedMeshComponent.SetLeaderPoseComponent` (`self.Left Shoulder Attachment`) (`self.Mesh`) false)
  (`SkinnedMeshComponent.SetLeaderPoseComponent` (`self.Right Elbow Attachment`) (`self.Mesh`) false)
  (`SkinnedMeshComponent.SetLeaderPoseComponent` (`self.Left Elbow Attachment`) (`self.Mesh`) false)
  (`SkinnedMeshComponent.SetLeaderPoseComponent` (`self.Left Knee Attachment`) (`self.Mesh`) false)
  (`SkinnedMeshComponent.SetLeaderPoseComponent` (`self.Right Knee Attachment`) (`self.Mesh`) false)
  (set `self.DamagedParticleAttachment` (`self.Mesh`))
  (`SceneComponent.K2_AttachToComponent` (`self.PopUpLocationComponent`) (`self.Head`) "None" "KeepWorld" "KeepWorld" "KeepWorld" true))