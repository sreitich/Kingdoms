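; Pyromancer mage piece whose active ability plays a power-up animation on a chosen target's encounter.
; On activation it saves attacker and target to the match GameState, then disables each player's input and zooms their cameras onto both pieces.
; A multicast from the server-owned piece then sets UsingActive on its anim Blueprint.
; Construction links modular body meshes to a master pose and configures damage particle and pop-up attachments.
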(event `Multicast_AnimatePyroPowerUp`
  ;[1 1 1] Animate the Pyromancer's power-up ability. Pieces are owned by the server so they can call RPCs.
  (bind _asbase_anim_bp (cast `/Game/Animations/Parent/BaseAnimBP` (`SkeletalMeshComponent.GetAnimInstance` (`self.Mesh`))))
  (set `AnimInstance_Parent.bUsingActive` true _asbase_anim_bp))

(event `self.BP_OnActiveAbility`
  (params (Target :type "ParentPiece Object Reference"))
  ;[1 1 1] Save the target in the game state to be used later when starting the attack.
  (bind _asbp_match_game_state_base (cast `/Game/Blueprints/Framework/Match/BP_Match_GameStateBase` (`GameplayStatics.GetGameState`)))
  (set `Match_GameStateBase.CurrentAttackInfo` (make `AttackInfo` self Target) _asbp_match_game_state_base)
  (bind _asbp_match_player_pawn (`/Game/Blueprints/Libraries/ActorMacroLibrary.Execute For Each Player's Pawn`)
    (:`Completed`
      ;[1 1 1] Animate the Pyromancer's power-up ability. Pieces are owned by the server so they can call RPCs.
      (`self.Multicast_AnimatePyroPowerUp`))
    (:`For Each Pawn...`
      ;[1 1 1] Disable each client's input.
      (`/Game/Blueprints/Framework/Match/BP_Match_PlayerPawn.Client_DisablePlayerInput` _asbp_match_player_pawn true)
      (bind _asbp_match_game_state_base_2 (cast `/Game/Blueprints/Framework/Match/BP_Match_GameStateBase` (`GameplayStatics.GetGameState`)))
      (bind (_currentattackinfo_attacker _currentattackinfo_defender) (break `AttackInfo` (`Match_GameStateBase.CurrentAttackInfo` _asbp_match_game_state_base_2)))
      ;[1 1 1] Zoom both players into the attacker and their target.
      (`Match_PlayerPawn.Client_MovePlayerCamera` _asbp_match_player_pawn _currentattackinfo_attacker _currentattackinfo_defender false))))

(fn `UserConstructionScript`
  (`SkinnedMeshComponent.SetLeaderPoseComponent` (`self.Head`) (`self.Mesh`) false)
  (`SkinnedMeshComponent.SetLeaderPoseComponent` (`self.Torso`) (`self.Mesh`) false)
  (`SkinnedMeshComponent.SetLeaderPoseComponent` (`self.Left Leg`) (`self.Mesh`) false)
  (`SkinnedMeshComponent.SetLeaderPoseComponent` (`self.Upper Left Arm`) (`self.Mesh`) false)
  (`SkinnedMeshComponent.SetLeaderPoseComponent` (`self.Hips`) (`self.Mesh`) false)
  (`SkinnedMeshComponent.SetLeaderPoseComponent` (`self.Right Leg`) (`self.Mesh`) false)
  (`SkinnedMeshComponent.SetLeaderPoseComponent` (`self.Lower Left Arm`) (`self.Mesh`) false)
  (`SkinnedMeshComponent.SetLeaderPoseComponent` (`self.Lower Right Arm`) (`self.Mesh`) false)
  (`SkinnedMeshComponent.SetLeaderPoseComponent` (`self.Left Hand`) (`self.Mesh`) false)
  (`SkinnedMeshComponent.SetLeaderPoseComponent` (`self.Right Hand`) (`self.Mesh`) false)
  (`SkinnedMeshComponent.SetLeaderPoseComponent` (`self.Upper Right Arm`) (`self.Mesh`) false)
  (`SkinnedMeshComponent.SetLeaderPoseComponent` (`self.Hood`) (`self.Mesh`) false)
  (`SkinnedMeshComponent.SetLeaderPoseComponent` (`self.Facial Hair`) (`self.Mesh`) false)
  (`SkinnedMeshComponent.SetLeaderPoseComponent` (`self.Eyebrows`) (`self.Mesh`) false)
  (set `self.DamagedParticleAttachment` (`self.Torso`))
  (`SceneComponent.K2_AttachToComponent` (`self.PopUpLocationComponent`) (`self.Head`) "None" "KeepWorld" "KeepWorld" "KeepWorld" true))