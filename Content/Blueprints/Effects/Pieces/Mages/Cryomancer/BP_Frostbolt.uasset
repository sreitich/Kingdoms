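; Frostbolt effect actor for the Cryomancer piece's active ability, which scales in on spawn and fades away by scale on impact.
; Each impact timeline update also spawns a splash emitter at the target and looks up the Cryomancer's data row.
; It then has the server add a hostile, timed strength and armor modifier through piece networking.
; An ice effect actor spawns attached to the target's mesh.
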(event `self.ReceiveBeginPlay`
  ;[1 1 1] Give the frostbolt a small pop-up animation.
  (bind (_direction _size) (`Timeline|SpawnTimeline` :!via `PlayFromStart`)
    (:`Update`
      (`self.SetActorScale3D` (`KismetMathLibrary.Conv_DoubleToVector` _size)))))

(event `self.OnImpact`
  (bind _returnvalue (`self.K2_GetActorLocation` (`self.Target`)))
  ;[1 1 1] Give the frostbolt a fade-away animation and create an impact effect.
  (bind (_direction _size) (`Timeline|ImpactTimeline`)
    (:`Update`
      (`self.SetActorScale3D` (`KismetMathLibrary.Conv_DoubleToVector` _size))
      (`GameplayStatics.SpawnEmitterAtLocation` "/Game/Assets/FantasyFX/Particles/Splash/P_Splash_Impact.P_Splash_Impact" _returnvalue (`KismetMathLibrary.FindLookAtRotation` (`self.K2_GetActorLocation`) _returnvalue) (0.75 0.75 0.75))
      ;[1 1 1] Create the active ability's modifier to add to the target.
      (bind _ascryomancer (cast `Cryomancer` (`self.GetOwner`)))
      (bind _returnvalue_2 (`|GetDataTableRow` (`ParentPiece.PieceDataTable` _ascryomancer) (`ParentPiece.PieceID` _ascryomancer))
        (:`then`
          (bind _asparent_piece (cast `ParentPiece` (`self.Target`)))
          (bind _asmatch_player_pawn (cast `Match_PlayerPawn` (`Actor.Instigator` _asparent_piece)))
          ;[1 1 1] Add the modifier on the server.
          (if (`self.HasAuthority` (`self.GetOwner`))
            (bind (_piecename _classtype _rarity _basearmor _basestrength _piecedes _classref _piececardportrait _pieceinfophoto _attackpreviewphoto _activename) (break `PieceDataStruct` _returnvalue_2))
            (`PieceNetworkingComponent.Server_AddModifier` (`Match_PlayerPawn.GetPieceNetworkingComponent` _asmatch_player_pawn) _asparent_piece (make `Modifier` _ascryomancer "E_Hostile" _piecename _activename 0 (`Cryomancer.FrostboltStrengthChange` _ascryomancer) (`Cryomancer.FrostboltArmorChange` _ascryomancer) false (`Cryomancer.FrostboltFreezeDuration` _ascryomancer) false false) true))
          ;[1 1 1] Spawn a frostbolt ice effect for every client.
          (bind _returnvalue_3 (`|SpawnActorFromClass` "/Game/Blueprints/Effects/Pieces/Mages/Cryomancer/BP_FrostboltIce.BP_FrostboltIce_C" (`self.GetTransform` _asparent_piece) "AlwaysSpawn" "OverrideRootScale" _ascryomancer null))
          (`self.K2_AttachToComponent` _returnvalue_3 (`Character.Mesh` _asparent_piece) "Root" "KeepWorld" "KeepWorld" "KeepWorld" true))))))

(fn `UserConstructionScript`
  (`parent.UserConstructionScript`))