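; BP_Pyro_Fireball is a Pyromancer fireball effect actor that flies from its current location to a given destination.
; ActivateFireball records the start location, activates the particle system and plays a travel timeline.
; The timeline's Delta track feeds VInterpTo as DeltaTime from the fixed start, so it acts as blend alpha for non-swept movement.
; When the timeline finishes, particles and trails end and the actor destroys itself.
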(event `ActivateFireball`
  (params (Destination :type "Vector Structure"))
  (bind _particlesystem (`self.ParticleSystem`))
  (set `self.SpawnLocation` (`self.K2_GetActorLocation`))
  (`ActorComponent.Activate` _particlesystem true)
  (bind (_direction _delta) (`Timeline|Fireball Travel Timeline` :!via `PlayFromStart`)
    (:`Update`
      (`self.K2_SetActorLocation` (`KismetMathLibrary.VInterpTo` (`self.SpawnLocation`) Destination _delta 1.0)))
    (:`Finished`
      (`ActorComponent.Deactivate` _particlesystem)
      (`ParticleSystemComponent.EndTrails` _particlesystem)
      (`self.K2_DestroyActor`))))

(fn `UserConstructionScript`)