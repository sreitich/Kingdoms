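; BP_Guardian_Armor is an effect for the Guardian piece that grants a temporary armor buff to its target piece on impact.
; On the server, it reads the Guardian's piece and ability names from its data table row.
; It then sends an armor modifier, using the Guardian's buff value and duration, through the piece networking component of the target's instigating player pawn, with pop-ups enabled.
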(event `self.OnImpact`
  (bind _returnvalue (`self.GetOwner`))
  (if (`self.HasAuthority` _returnvalue)
    (bind _asguardian (cast `Guardian` _returnvalue))
    (bind _returnvalue_2 (`|GetDataTableRow` (`ParentPiece.PieceDataTable` _asguardian) (`ParentPiece.PieceID` _asguardian))
      (:`then`
        (bind _asparent_piece (cast `ParentPiece` (`self.Target`)))
        (bind _asmatch_player_pawn (cast `Match_PlayerPawn` (`Actor.Instigator` _asparent_piece)))
        (bind (_piecename _classtype _rarity _basearmor _basestrength _piecedes _classref _piececardportrait _pieceinfophoto _attackpreviewphoto _activename) (break `PieceDataStruct` _returnvalue_2))
        (`PieceNetworkingComponent.Server_AddModifier` (`Match_PlayerPawn.GetPieceNetworkingComponent` _asmatch_player_pawn) _asparent_piece (make `Modifier` _returnvalue "E_Friendly" _piecename _activename 0 0 (`Guardian.ArmorBuffValue` _asguardian) false (`Guardian.ArmorBuffDuration` _asguardian) true false) true)))))

(fn `UserConstructionScript`
  (`parent.UserConstructionScript`))