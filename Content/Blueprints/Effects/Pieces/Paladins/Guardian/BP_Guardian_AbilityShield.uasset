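; BP_Guardian_AbilityShield is the shield effect for the Guardian paladin piece's ability, popping up through a scale timeline on spawn.
; A random speed is written to a dynamic material on its sphere.
; When destroyed with ContinuePushDeath set, it spawns a replica with the same transform and speed to delay its visual death.
; The replica skips the pop-up, plays a shrink timeline and destroys itself without respawning.
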(event `self.ReceiveBeginPlay`
  ;[1 1 1] When spawned, give this shield a random speed.
  (`self.SetShieldSpeed` (`KismetMathLibrary.RandomFloatInRange` 0.25 0.6))
  ;[1 1 1] Interpolate this shield's size to give it a popping-up animation.
  (bind (_direction _delta) (`Timeline|Grow Timeline`)
    (:`Update`
      (`self.SetActorScale3D` (`KismetMathLibrary.Conv_DoubleToVector` _delta)))))

(event `SetShieldSpeed`
  (params (NewShieldSpeed :type "Float (double-precision)"))
  (bind _sphere (`self.Sphere`))
  ;[1 1 1] Set the shield's speed to the given value.
  (bind _returnvalue (`PrimitiveComponent.CreateDynamicMaterialInstance` _sphere 0 (`PrimitiveComponent.GetMaterial` _sphere 0) "None"))
  (bind _output_get (set `self.ShieldSpeed` NewShieldSpeed))
  (`MaterialInstanceDynamic.SetScalarParameterValue` _returnvalue "Speed_2" _output_get))

(event `self.ReceiveDestroyed`
  ;[1 1 1] When a request to destroy this actor is received, check if the destruction needs to be pushed back.
  (if (`self.bContinuePushDeath`)
    ;[1 1 1] If the actor's death needs to be pushed back, create an exact replica of it before destroying it.
    (bind _returnvalue (`|SpawnActorFromClass` "BP_Guardian_AbilityShield_C" (`self.GetTransform`) "AlwaysSpawn" "OverrideRootScale" null null))
    (`self.SetShieldSpeed` _returnvalue (`self.ShieldSpeed`)) ; Replicate the shield's speed.
    (`TimelineComponent.SetPlaybackPosition` (`/Game/Blueprints/Effects/Pieces/Paladins/Guardian/BP_Guardian_AbilityShield.Grow Timeline` _returnvalue) 0.5 false true) ; Prevent the replica from playing\na pop-up animation.
    ;[1 1 1] Make it so the exact replica does not push back its own destruction.
    (set `/Game/Blueprints/Effects/Pieces/Paladins/Guardian/BP_Guardian_AbilityShield.bContinuePushDeath` false _returnvalue)
    ;[1 1 1] Destroy the replica after a shrinking animation.
    (`self.PushDestroyActor` _returnvalue)))

(event `PushDestroyActor`
  ;[1 1 1] Play a shrinking animation when destroying an actor via a push request.
  (bind (_direction _delta) (`Timeline|Shrink Timeline` :!via `PlayFromStart`)
    (:`Update`
      (`self.SetActorScale3D` (`KismetMathLibrary.Conv_DoubleToVector` _delta)))
    (:`Finished`
      (`self.K2_DestroyActor`))))

(fn `UserConstructionScript`)