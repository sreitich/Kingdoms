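; BP_TrackingProjectile is an effect projectile that flies from its spawn point to a given destination.
; ActivateProjectile starts the particle system and a timeline whose Delta track feeds VInterpTo from the fixed start, acting as a lerp alpha without sweeping.
; Target is stored but does not steer the flight.
; When the timeline finishes, trails end, the empty OnImpact hook fires for overrides, and the actor destroys itself.
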(event `ActivateProjectile`
  (params (Destination :type "Vector Structure") (Target :type "Actor Object Reference"))
  (bind _particlesystem (`self.ParticleSystem`))
  (set `self.SpawnLocation` (`self.K2_GetActorLocation`))
  (set `self.Target` Target)
  (`ActorComponent.Activate` _particlesystem true)
  (bind (_direction _delta) (`Timeline|Projectile Travel Timeline` :!via `PlayFromStart`)
    (:`Update`
      (`self.K2_SetActorLocation` (`KismetMathLibrary.VInterpTo` (`self.SpawnLocation`) Destination _delta 1.0)))
    (:`Finished`
      (`ActorComponent.Deactivate` _particlesystem)
      (`ParticleSystemComponent.EndTrails` _particlesystem)
      (`self.OnImpact`)
      (`self.K2_DestroyActor`))))

(event `OnImpact`
  ;[1 1 1] Overridden
)

(fn `UserConstructionScript`)