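; Player pawn for a networked piece-based match, providing the spring-arm camera controls and running the scripted attack sequence between two pieces.
; Timelines drive view tilt, quarter-turn rotation and camera interpolation.
; The server stores attack info in the game state, positions pieces, then fans out camera, input, highlight and widget updates through each player's pawn.
; Animation notifies advance the sequence to strength-versus-armor outcome animations and final resolution of deaths, tiles and player state.
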(event `self.ReceiveBeginPlay`
  ;[1 1 1] This should always be 0.0, -30.0, 0.0 at the beginning of the game.
  (set `self.SpringArmRotation` (`SceneComponent.RelativeRotation` (`self.SpringArm`))))

(event `InputAction|MoveUp`
  (params (Key :type "Key Structure"))
  (bind (_springarmrotation_roll _springarmrotation_pitch _springarmrotation_yaw) (`KismetMathLibrary.BreakRotator` (`self.SpringArmRotation`)))
  ;[1 1 1] Switching between top-down and angled view.
  (:`Pressed`
    (set `self.bIsTopDown` true)
    (bind (_direction _pitch) (`Timeline|Move UpDown Timeline` :!label _label)
      (:`Update`
        (bind _returnvalue (* _pitch -90.0))
        (`SceneComponent.K2_SetRelativeRotation` (`self.SpringArm`) (`KismetMathLibrary.MakeRotator` _springarmrotation_roll _returnvalue _springarmrotation_yaw) false false))
      (:`Finished`
        (set `self.SpringArmRotation` (`KismetMathLibrary.MakeRotator` _springarmrotation_roll _returnvalue _springarmrotation_yaw))))))

(event `InputAction|MoveDown`
  (params (Key :type "Key Structure"))
  ;[1 1 1] Switching between top-down and angled view.
  (:`Pressed`
    (set `self.bIsTopDown` false)
    (goto _label :!via `Reverse`)))

(event `InputAxis|Zoom`
  (params (AxisValue :type "Float (single-precision)"))
  (bind _springarm (`self.SpringArm`))
  ;[1 1 1] Zooming in and out.
  (bind _output_get (set `self.NewTargetArmLength` (`KismetMathLibrary.FClamp` (+ (* AxisValue (`self.ZoomSpeed`)) (`self.NewTargetArmLength`)) 300.0 2000.0)))
  (set `SpringArmComponent.TargetArmLength` (`KismetMathLibrary.FInterpTo` (`SpringArmComponent.TargetArmLength` _springarm) _output_get (`GameplayStatics.GetWorldDeltaSeconds`) 15.0) _springarm))

(event `InputAction|MoveRight`
  (params (Key :type "Key Structure"))
  (bind (_springarmrotation_roll _springarmrotation_pitch _springarmrotation_yaw) (`KismetMathLibrary.BreakRotator` (`self.SpringArmRotation`)))
  (bind (_springarmrotation_roll_2 _springarmrotation_pitch_2 _springarmrotation_yaw_2) (`KismetMathLibrary.BreakRotator` (`self.SpringArmRotation`)))
  ;[1 1 1] Rotating to the right.
  (:`Pressed`
    (if (not (`self.Moving`))
      (set `self.Moving` true)
      (bind (_direction _yaw) (`Timeline|Move Right Timeline` :!via `PlayFromStart`)
        (:`Update`
          (`SceneComponent.K2_SetRelativeRotation` (`self.SpringArm`) (`KismetMathLibrary.MakeRotator` _springarmrotation_roll _springarmrotation_pitch (+ (* _yaw 90.0) _springarmrotation_yaw)) false false))
        (:`Finished`
          (set `self.SpringArmRotation` (`KismetMathLibrary.MakeRotator` _springarmrotation_roll_2 _springarmrotation_pitch_2 (- _springarmrotation_yaw_2 90.0)))
          (set `self.Moving` false))))))

(event `InputAction|MoveLeft`
  (params (Key :type "Key Structure"))
  (bind (_springarmrotation_roll _springarmrotation_pitch _springarmrotation_yaw) (`KismetMathLibrary.BreakRotator` (`self.SpringArmRotation`)))
  (bind (_springarmrotation_roll_2 _springarmrotation_pitch_2 _springarmrotation_yaw_2) (`KismetMathLibrary.BreakRotator` (`self.SpringArmRotation`)))
  ;[1 1 1] Rotating to the left.
  (:`Pressed`
    (if (not (`self.Moving`))
      (set `self.Moving` true)
      (bind (_direction _yaw) (`Timeline|Move Left Timeline` :!via `PlayFromStart`)
        (:`Update`
          (`SceneComponent.K2_SetRelativeRotation` (`self.SpringArm`) (`KismetMathLibrary.MakeRotator` _springarmrotation_roll _springarmrotation_pitch (+ (* _yaw 90.0) _springarmrotation_yaw)) false false))
        (:`Finished`
          (set `self.SpringArmRotation` (`KismetMathLibrary.MakeRotator` _springarmrotation_roll_2 _springarmrotation_pitch_2 (+ _springarmrotation_yaw_2 90.0)))
          (set `self.Moving` false))))))

(event `Server_AnimatePiecesAttacks`
  ;[1 0 0] Initializes the attack sequence and animates both pieces' attacks when finished. Animation notifies in the attack animations are used to continue the attack sequence.
  ;;[1 1 1 1 14] Move each client's pawn's camera to a target transform depending on the location of the pieces. This animates both pieces' attacks when the camera has finished moving.
  (bind _asbp_match_game_state_base (cast `/Game/Blueprints/Framework/Match/BP_Match_GameStateBase` (`GameplayStatics.GetGameState`)))
  (if (not (`/Game/Blueprints/Framework/Match/BP_Match_GameStateBase.PiecesAnimated` _asbp_match_game_state_base))
    (set `/Game/Blueprints/Framework/Match/BP_Match_GameStateBase.PiecesAnimated` true _asbp_match_game_state_base)
    (`self.Multicast_AnimatePiecesAttacks`)))

(event `Multicast_AnimatePiecesAttacks`
  ;[1 0 0] Initializes the attack sequence and animates both pieces' attacks when finished. Animation notifies in the attack animations are used to continue the attack sequence.
  ;;[1 1 1 1 14] Move each client's pawn's camera to a target transform depending on the location of the pieces. This animates both pieces' attacks when the camera has finished moving.
  (bind _asbp_match_game_state_base (cast `/Game/Blueprints/Framework/Match/BP_Match_GameStateBase` (`GameplayStatics.GetGameState`)))
  (bind (_currentattackinfo_attacker _currentattackinfo_defender _currentattackinfo_bmoveto _currentattackinfo_bdefenderfights) (break `AttackInfo` (`/Game/Blueprints/Framework/Match/BP_Match_GameStateBase.CurrentAttackInfo` _asbp_match_game_state_base)))
  (bind _asbase_anim_bp (cast `/Game/Animations/Parent/BaseAnimBP` (`SkeletalMeshComponent.GetAnimInstance` (`Character.Mesh` _currentattackinfo_attacker))))
  (set `AnimInstance_Parent.bAttacking` true _asbase_anim_bp)
  (bind _asbase_anim_bp_2 (cast `/Game/Animations/Parent/BaseAnimBP` (`SkeletalMeshComponent.GetAnimInstance` (`Character.Mesh` _currentattackinfo_defender))))
  (if _currentattackinfo_bdefenderfights
    (set `AnimInstance_Parent.bAttacking` true _asbase_anim_bp_2)
    (else
      (set `AnimInstance_Parent.bTakingDamage` false _asbase_anim_bp_2))))

(event `Multicast_AnimateDamageEffects`
  (params (AttackerDamage :type Boolean))
  ;[1 0 0] Initializes the attack sequence and animates both pieces' attacks when finished. Animation notifies in the attack animations are used to continue the attack sequence.
  ;;[1 1 1 1 14] Move each client's pawn's camera to a target transform depending on the location of the pieces. This animates both pieces' attacks when the camera has finished moving.
  (bind _asbp_match_game_state_base (cast `/Game/Blueprints/Framework/Match/BP_Match_GameStateBase` (`GameplayStatics.GetGameState`)))
  (if (not AttackerDamage)
    (bind (_currentattackinfo_attacker _currentattackinfo_defender) (break `AttackInfo` (`/Game/Blueprints/Framework/Match/BP_Match_GameStateBase.CurrentAttackInfo` _asbp_match_game_state_base)))
    (bind (_damagedparticletransform_location _damagedparticletransform_rotation _damagedparticletransform_scale) (`KismetMathLibrary.BreakTransform` (`ParentPiece.DamagedParticleTransform` _currentattackinfo_attacker)))
    (`GameplayStatics.SpawnEmitterAttached` (`ParentPiece.DamagedParticle` _currentattackinfo_attacker) (`ParentPiece.DamagedParticleAttachment` _currentattackinfo_attacker) "None" _damagedparticletransform_location _damagedparticletransform_rotation _damagedparticletransform_scale)
    (else
      (bind (_damagedparticletransform_location_2 _damagedparticletransform_rotation_2 _damagedparticletransform_scale_2) (`KismetMathLibrary.BreakTransform` (`ParentPiece.DamagedParticleTransform` _currentattackinfo_defender)))
      (`GameplayStatics.SpawnEmitterAttached` (`ParentPiece.DamagedParticle` _currentattackinfo_defender) (`ParentPiece.DamagedParticleAttachment` _currentattackinfo_defender) "None" _damagedparticletransform_location_2 _damagedparticletransform_rotation_2 _damagedparticletransform_scale_2))))

(event `Client_FlashHighlight`
  (params (Piece :type "ParentPiece Object Reference") (Color :type "LinearColor Structure") (Brightness :type "Float (double-precision)") (Duration :type "Float (double-precision)"))
  ;[1 0 0] Initializes the attack sequence and animates both pieces' attacks when finished. Animation notifies in the attack animations are used to continue the attack sequence.
  ;;[1 1 1 1 14] Flash both pieces white to indicate which ones are fighting.
  (`ParentPiece.FlashHighlight` Piece Color Brightness Duration))

(event `self.Server_Attack_BP`
  (params (InInfo :type "AttackInfo Structure"))
  ;[1 0 0] Initializes the attack sequence and animates both pieces' attacks when finished. Animation notifies in the attack animations are used to continue the attack sequence.
  ;;[1 1 1 1 14] Save the attack information in the game state to use later.
  (bind _asbp_match_game_state_base (cast `/Game/Blueprints/Framework/Match/BP_Match_GameStateBase` (`GameplayStatics.GetGameState`)))
  (bind _output_get (set `/Game/Blueprints/Framework/Match/BP_Match_GameStateBase.CurrentAttackInfo` (make `AttackInfo` InInfo_Attacker InInfo_Defender InInfo_bMoveTo InInfo_bDefenderFights InInfo_bTakePlace) _asbp_match_game_state_base))
  ;;[1 1 1 1 14] Disable input for each player's pawn.
  (bind _asbp_match_player_pawn (`self.Execute for Each Player's Pawn`)
    (:`Completed`
      (bind (_attacker _defender _bmoveto _bdefenderfights) (break `AttackInfo` _output_get))
      ;;[1 1 1] Rotate both pieces to face each other.
      (set `self.InitialAttackerRotation` (`self.K2_GetActorRotation` _attacker))
      (set `self.InitialDefenderRotation` (`self.K2_GetActorRotation` _defender))
      (`self.K2_SetActorRotation` _attacker (`KismetMathLibrary.FindLookAtRotation` (`self.K2_GetActorLocation` _attacker) (`self.K2_GetActorLocation` _defender)) false)
      (`self.K2_SetActorRotation` _defender (`KismetMathLibrary.FindLookAtRotation` (`self.K2_GetActorLocation` _defender) (`self.K2_GetActorLocation` _attacker)) false)
      ;;[1 1 1 1 14] Ensure that the pieces are close enough, and move the attacker to the defender if necessary.
      (if (> (`self.GetDistanceTo` _attacker _defender) 300.0)
        (setmembers `AttackInfo` :`StructRef` _output_get :`bMoveTo` true) ; Save a variable that determines whether the piece had to be moved or not.
        (bind _asbp_piece_aicontroller (cast `/Game/Blueprints/Pieces/BP_PieceAIController` (`self.GetOwner` _attacker)))
        (set `PieceAIController.bResetAfterMove` false _asbp_piece_aicontroller) ; Make sure that this piece doesn't\nreset its direction after moving.
        (`AITask_MoveTo.AIMoveTo` _asbp_piece_aicontroller (`self.K2_GetActorLocation` _defender) null (`self.Minimum Attacking Distance`)
          (:`OnMoveFinished`
            _))
        (else
          (setmembers `AttackInfo` :`StructRef` _output_get :`bMoveTo` false) ; Save a variable that determines whether the piece had to be moved or not.
        ))
      ;;[1 1 1 1 14] Move each client's pawn's camera to a target transform depending on the location of the pieces. This animates both pieces' attacks when the camera has finished moving.
      (bind _asbp_match_player_pawn_2 (`self.Execute for Each Player's Pawn`)
        (:`For Each Pawn...`
          (`self.Client_MovePlayerCamera` _asbp_match_player_pawn_2 _attacker _defender false) ; When this finishes, the pieces are animated.\nThe attack sequence continues with animation\nnotifies.
          (`self.Server_AnimatePiecesAttacks` _asbp_match_player_pawn_2) ; Animates and spawns effects for the pieces' attacks.
          ;;[1 1 1 1 14] Flash both pieces white to indicate which ones are fighting.
          (`self.Client_FlashHighlight` _asbp_match_player_pawn_2 _attacker (struct :`R` 1.0 :`G` 1.0 :`B` 1.0 :`A` 1.0) 15.0 1.0)
          (`self.Client_FlashHighlight` _asbp_match_player_pawn_2 _defender (struct :`R` 1.0 :`G` 1.0 :`B` 1.0 :`A` 1.0) 15.0 1.0)
          ;;[1 1 1 1 14] Creates and plays the animation for the attack graphic widget, depending on whether or not the defender fights back.
          (`self.Client_UpdateAttackGraphicWidget` _asbp_match_player_pawn_2 false _attacker _defender)
          (if _bdefenderfights
            (`self.Client_AnimateAttackGraphicWidget` _asbp_match_player_pawn_2 "E_NeutralFightInitiation")
            (else
              (`self.Client_AnimateAttackGraphicWidget` _asbp_match_player_pawn_2 "E_AttackerFightInitiation"))))))
    (:`For Each Pawn...`
      (`self.Client_DisablePlayerInput` _asbp_match_player_pawn true))))

(event `Client_DisablePlayerInput`
  (params (DisableInput :type Boolean))
  ;[1 0 0] Initializes the attack sequence and animates both pieces' attacks when finished. Animation notifies in the attack animations are used to continue the attack sequence.
  ;;[1 1 1 1 14] Disable input for each player's pawn.
  (bind _asplayer_controller (cast `PlayerController` (`self.GetController`)))
  (if DisableInput
    (`self.DisableInput` _asplayer_controller)
    (else
      (`self.EnableInput` _asplayer_controller))))

(event `self.InterpolatePlayerCamera`
  (params (TargetLocation :type "Vector Structure") (TargetRotation :type "Rotator Structure") (TargetArmLength :type "Float (single-precision)") (bReverse :type Boolean))
  (bind (_originalviewtransform_location _originalviewtransform_rotation) (`KismetMathLibrary.BreakTransform` (`self.OriginalViewTransform`)))
  (bind _springarm (`self.SpringArm`))
  ;[1 0 0] Initializes the attack sequence and animates both pieces' attacks when finished. Animation notifies in the attack animations are used to continue the attack sequence.
  ;;[1 1 1 1 14] Move each client's pawn's camera to a target transform depending on the location of the pieces. This animates both pieces' attacks when the camera has finished moving.
  (`TimelineComponent.SetPlayRate` (`self.Interpolate Player Camera Timeline`) (/ (`self.CameraInterpDuration`) 0.5)) ; Playrate can be adjusted manually
  (if (not bReverse)
    (bind (_direction _delta) (`Timeline|Interpolate Player Camera Timeline` :!label _label)
      (:`Update`
        (`SceneComponent.K2_SetWorldLocation` _springarm (`KismetMathLibrary.VInterpTo` _originalviewtransform_location TargetLocation _delta 1.0) false false)
        (`SceneComponent.K2_SetWorldRotation` _springarm (`KismetMathLibrary.RInterpTo` _originalviewtransform_rotation TargetRotation _delta 1.0) false false)
        (set `SpringArmComponent.TargetArmLength` (`KismetMathLibrary.FInterpTo` (`self.OriginalCameraArmLength`) TargetArmLength _delta 1.0) _springarm)))
    (else
      (goto _label :!via `Reverse`))))

(event `Client_AnimateAttackGraphicWidget`
  (params (AnimationToPlay :type "EAttackGraphicAnimation Enum" :default "E_NeutralFightInitiation"))
  ;[1 0 0] Initializes the attack sequence and animates both pieces' attacks when finished. Animation notifies in the attack animations are used to continue the attack sequence.
  ;;[1 1 1 1 14] Creates and plays the animation for the attack graphic widget, depending on whether or not the defender fights back.
  (bind _asbp_match_player_controller (cast `/Game/Blueprints/Framework/Match/BP_Match_PlayerController` (`self.GetController`)))
  (`Match_PlayerController.PlayAttackGraphicAnimation` _asbp_match_player_controller AnimationToPlay))

(event `Client_UpdateAttackGraphicWidget`
  (params (bDestroy :type Boolean) (Attacker :type "ParentPiece Object Reference") (Defender :type "ParentPiece Object Reference"))
  ;[1 0 0] Initializes the attack sequence and animates both pieces' attacks when finished. Animation notifies in the attack animations are used to continue the attack sequence.
  ;;[1 1 1 1 14] Creates and plays the animation for the attack graphic widget, depending on whether or not the defender fights back.
  (bind _asbp_match_player_controller (cast `/Game/Blueprints/Framework/Match/BP_Match_PlayerController` (`self.GetController`)))
  (`Match_PlayerController.UpdateAttackGraphicWidget` _asbp_match_player_controller bDestroy Attacker Defender) ; Create and initialize the attack graphic widget.
)

(event `Server_AnimateAttackOutcome`
  ;[1 0.05 0] When both pieces finish their attack animation, call another multicast to play a new animation on each piece depending on the outcome of this attack.
  (bind _attackresult (`self.GetCurrentAttackOutcome`))
  (`self.Multicast_AnimateAttackResults` _attackresult))

(event `Multicast_AnimateAttackResults`
  (params (AttackResult :type "EAttackResult Enum" :default "E_AttackerSurvivesDefenderDies"))
  ;[1 0.2 0] Animate the attacker and defender on each client depending on the attack result.
  (bind _asbp_match_game_state_base (cast `/Game/Blueprints/Framework/Match/BP_Match_GameStateBase` (`GameplayStatics.GetGameState`)))
  (bind (_currentattackinfo_attacker _currentattackinfo_defender) (break `AttackInfo` (`/Game/Blueprints/Framework/Match/BP_Match_GameStateBase.CurrentAttackInfo` _asbp_match_game_state_base)))
  (bind _asbase_anim_bp (cast `/Game/Animations/Parent/BaseAnimBP` (`SkeletalMeshComponent.GetAnimInstance` (`Character.Mesh` _currentattackinfo_attacker))))
  (switch `EAttackResult` AttackResult
    (:`E_AttackerSurvivesDefenderDies`
      (set `AnimInstance_Parent.bCelebrating` true _asbase_anim_bp))
    (:`E_DefenderSurvivesAttackerDies`
      (set `AnimInstance_Parent.bDying` true _asbase_anim_bp))
    (:`E_AttackerDiesDefenderDies`
      (set `AnimInstance_Parent.bDying` true _asbase_anim_bp))
    (:`E_AttackerSurvivesDefenderSurvives`
      (set `AnimInstance_Parent.bDeadlocking` true _asbase_anim_bp))
    (:`E_DefenderSurvives`
      (set `AnimInstance_Parent.bDeadlocking` true _asbase_anim_bp)))
  (bind _asbase_anim_bp_2 (cast `/Game/Animations/Parent/BaseAnimBP` (`SkeletalMeshComponent.GetAnimInstance` (`Character.Mesh` _currentattackinfo_defender))))
  (switch `EAttackResult` AttackResult
    (:`E_AttackerSurvivesDefenderDies`
      (set `AnimInstance_Parent.bDying` true _asbase_anim_bp_2))
    (:`E_DefenderSurvivesAttackerDies`
      (set `AnimInstance_Parent.bCelebrating` true _asbase_anim_bp_2))
    (:`E_AttackerDiesDefenderDies`
      (set `AnimInstance_Parent.bDying` true _asbase_anim_bp_2))
    (:`E_AttackerSurvivesDefenderSurvives`
      (set `AnimInstance_Parent.bDeadlocking` true _asbase_anim_bp_2))
    (:`E_DefenderSurvives`
      _))
  ;[1 0.2 0] Play an attack graphic animation depending on the result of the attack.
  (bind _asbp_match_player_pawn (`self.Execute for Each Player's Pawn`)
    (:`For Each Pawn...`
      (switch `EAttackResult` AttackResult
        (:`E_AttackerSurvivesDefenderDies`
          (`self.Client_AnimateAttackGraphicWidget` _asbp_match_player_pawn "E_DefenderDeath"))
        (:`E_DefenderSurvivesAttackerDies`
          (`self.Client_AnimateAttackGraphicWidget` _asbp_match_player_pawn "E_AttackerDeath"))
        (:`E_AttackerDiesDefenderDies`
          (`self.Client_AnimateAttackGraphicWidget` _asbp_match_player_pawn "E_AttackerDeath")
          (`self.Client_AnimateAttackGraphicWidget` _asbp_match_player_pawn "E_DefenderDeath"))
        (:`E_AttackerSurvivesDefenderSurvives`
          (`self.Client_AnimateAttackGraphicWidget` _asbp_match_player_pawn "E_AttackerDeadlock")
          (`self.Client_AnimateAttackGraphicWidget` _asbp_match_player_pawn "E_DefenderDeadlock"))
        (:`E_DefenderSurvives`
          (`self.Client_AnimateAttackGraphicWidget` _asbp_match_player_pawn "E_AttackerDeadlock")))
      ;[1 0.2 0] Flash a highlight over both pieces depending on the result of the attack.
      (bind _asbp_match_player_pawn_2 (`self.Execute for Each Player's Pawn`)
        (:`For Each Pawn...`
          (switch `EAttackResult` AttackResult
            (:`E_AttackerSurvivesDefenderDies`
              (`self.Client_FlashHighlight` _asbp_match_player_pawn_2 _currentattackinfo_attacker (struct :`G` 0.5 :`A` 1.0) 15.0 1.0)
              (`self.Client_FlashHighlight` _asbp_match_player_pawn_2 _currentattackinfo_defender (struct :`R` 0.5 :`A` 1.0) 15.0 1.0))
            (:`E_DefenderSurvivesAttackerDies`
              (`self.Client_FlashHighlight` _asbp_match_player_pawn_2 _currentattackinfo_attacker (struct :`R` 0.5 :`A` 1.0) 15.0 1.0)
              (`self.Client_FlashHighlight` _asbp_match_player_pawn_2 _currentattackinfo_defender (struct :`G` 0.5 :`A` 1.0) 15.0 1.0))
            (:`E_AttackerDiesDefenderDies`
              (`self.Client_FlashHighlight` _asbp_match_player_pawn_2 _currentattackinfo_attacker (struct :`R` 0.5 :`A` 1.0) 15.0 1.0)
              (`self.Client_FlashHighlight` _asbp_match_player_pawn_2 _currentattackinfo_defender (struct :`R` 0.5 :`A` 1.0) 15.0 1.0))
            (:`E_AttackerSurvivesDefenderSurvives`
              (`self.Client_FlashHighlight` _asbp_match_player_pawn_2 _currentattackinfo_attacker (struct :`R` 0.5 :`G` 0.5 :`A` 1.0) 15.0 1.0)
              (`self.Client_FlashHighlight` _asbp_match_player_pawn_2 _currentattackinfo_defender (struct :`R` 0.5 :`G` 0.5 :`A` 1.0) 15.0 1.0))
            (:`E_DefenderSurvives`
              (`self.Client_FlashHighlight` _asbp_match_player_pawn_2 _currentattackinfo_attacker (struct :`R` 0.5 :`G` 0.5 :`A` 1.0) 15.0 1.0)
              (`self.Client_FlashHighlight` _asbp_match_player_pawn_2 _currentattackinfo_defender (struct :`R` 0.5 :`G` 0.5 :`A` 1.0) 15.0 1.0))))))))

(event `Server_ResolveAttack`
  ;[1 0.4 0] Reset the match, both players, and surviving pieces to before the attack sequence activated.
  (bind _asbp_match_player_pawn (`self.Execute for Each Player's Pawn`) ; Reset each player.
    (:`Completed`
      (bind _asbp_match_game_state_base (cast `/Game/Blueprints/Framework/Match/BP_Match_GameStateBase` (`GameplayStatics.GetGameState`)))
      (bind _currentattackinfo_attacker (break `AttackInfo` (`/Game/Blueprints/Framework/Match/BP_Match_GameStateBase.CurrentAttackInfo` _asbp_match_game_state_base)))
      (bind _asmatch_player_state (cast `Match_PlayerState` (`Pawn.PlayerState` (`self.GetInstigator` _currentattackinfo_attacker))))
      (`Match_PlayerState.Server_SetPlayerStatus` _asmatch_player_state "E_SelectingPiece")
      (bind (_attackresult _castedgamestate) (`self.GetCurrentAttackOutcome`))
      (switch `EAttackResult` _attackresult
        (:`E_AttackerSurvivesDefenderDies`
          (bind (_currentattackinfo_attacker_2 _currentattackinfo_defender _currentattackinfo_bmoveto _currentattackinfo_bdefenderfights _currentattackinfo_btakeplace) (break `AttackInfo` (`/Game/Blueprints/Framework/Match/BP_Match_GameStateBase.CurrentAttackInfo` _castedgamestate)))
          (if _currentattackinfo_btakeplace
            (bind _asmatch_player_controller (cast `Match_PlayerController` (`self.GetController`)))
            (bind _asbp_piece_aicontroller (cast `/Game/Blueprints/Pieces/BP_PieceAIController` (`self.GetController` _currentattackinfo_attacker_2)))
            (set `PieceAIController.bResetAfterMove` true _asbp_piece_aicontroller) ; Reset this piece's rotation after it finishes moving.
            (`ServerCommunicationComponent.MovePieceToTile_Server` (`Match_PlayerController.ServerCommunicationComponent` _asmatch_player_controller) _currentattackinfo_attacker_2 (`ParentPiece.GetCurrentTile` _currentattackinfo_defender) false))
          (`self.PieceDiedResolution` _currentattackinfo_defender (not _currentattackinfo_btakeplace)))
        (:`E_DefenderSurvivesAttackerDies`
          (`self.PieceDiedResolution` _currentattackinfo_attacker_2 true))
        (:`E_AttackerDiesDefenderDies`
          (`self.PieceDiedResolution` _currentattackinfo_defender true)
          (`self.PieceDiedResolution` _currentattackinfo_attacker_2 true))
        (:`E_AttackerSurvivesDefenderSurvives`
          (if _currentattackinfo_bmoveto :!label _label_2
            (`self.Server_SetResetAfterMove` _currentattackinfo_attacker_2 true) ; Reset this piece's rotation after it finishes moving.
            (bind _asbp_piece_aicontroller_2 (cast `/Game/Blueprints/Pieces/BP_PieceAIController` (`self.GetController` _currentattackinfo_attacker_2)))
            (`AITask_MoveTo.AIMoveTo` _asbp_piece_aicontroller_2 (`self.K2_GetActorLocation` (`ParentPiece.GetCurrentTile` _currentattackinfo_attacker_2)) null -1.0 "Disable"
              (:`then`
                _))))
        (:`E_DefenderSurvives`
          (goto _label_2)))
      (bind _asbp_match_game_state_base_2 (cast `/Game/Blueprints/Framework/Match/BP_Match_GameStateBase` (`GameplayStatics.GetGameState`)))
      (bind (_currentattackinfo_attacker_3 _currentattackinfo_defender_2) (break `AttackInfo` (`/Game/Blueprints/Framework/Match/BP_Match_GameStateBase.CurrentAttackInfo` _asbp_match_game_state_base_2)))
      (`/Engine/EditorBlueprintResources/StandardMacros.IsValid` _currentattackinfo_attacker_3
        (:`Is Valid`
          (`ParentPiece.Server_ResetPieceRotation` _currentattackinfo_attacker_3) ; Reset the attacker's rotation\nif it survived.
        )
        (:`Is Not Valid`
          _))
      (`/Engine/EditorBlueprintResources/StandardMacros.IsValid` _currentattackinfo_defender_2
        (:`Is Valid`
          (`ParentPiece.Server_ResetPieceRotation` _currentattackinfo_defender_2) ; Reset the attacker's rotation\nif it survived.
        )
        (:`Is Not Valid`)))
    (:`For Each Pawn...`
      (`self.Client_UpdateAttackGraphicWidget` _asbp_match_player_pawn true null null) ; Destroy the attack graphic widget
      (`self.Client_DisablePlayerInput` _asbp_match_player_pawn false) ; Enable input for this client.
      (bind _asbp_match_game_state_base_3 (cast `/Game/Blueprints/Framework/Match/BP_Match_GameStateBase` (`GameplayStatics.GetGameState`)))
      (bind (_currentattackinfo_attacker_4 _currentattackinfo_defender_3) (break `AttackInfo` (`/Game/Blueprints/Framework/Match/BP_Match_GameStateBase.CurrentAttackInfo` _asbp_match_game_state_base_3)))
      (`self.Client_MovePlayerCamera` _asbp_match_player_pawn _currentattackinfo_attacker_4 _currentattackinfo_defender_3 true))))

(event `PieceDiedResolution`
  (params (DeadPiece :type "ParentPiece Object Reference") (ClearOccupiedPiece :type Boolean))
  ;[1 0.4 0] Reset the match, both players, and surviving pieces to before the attack sequence activated.
  (bind _asmatch_player_state (cast `Match_PlayerState` (`Pawn.PlayerState` (`Actor.Instigator` DeadPiece))))
  (`KismetArrayLibrary.Array_RemoveItem` (`Match_PlayerState.OwnedPieces` _asmatch_player_state) DeadPiece)
  (if ClearOccupiedPiece
    (`BoardTile.SetOccupyingPiece` (`ParentPiece.GetCurrentTile` DeadPiece) null))
  (`self.K2_DestroyActor` DeadPiece))

(fn `IdentifyAttackResult`
  (params (Attacker :type "ParentPiece Object Reference") (Defender :type "ParentPiece Object Reference") (DefenderFights :type Boolean))
  (returns (AttackResult :type "EAttackResult Enum") (`Casted Game State` :type Boolean))
  (locals (AttackerStrength :type Integer) (AttackerArmor :type Integer) (DefenderStrength :type Integer) (DefenderArmor :type Integer))
  ;[1 1 1 1 14] Save the attacker and defender info in local variables to use more easily.
  (set `local.AttackerStrength` (`ParentPiece.GetCurrentStrength` Attacker))
  (set `local.AttackerArmor` (`ParentPiece.GetCurrentArmor` Attacker))
  (set `local.DefenderStrength` (`ParentPiece.GetCurrentStrength` Defender))
  (set `local.DefenderArmor` (`ParentPiece.GetCurrentArmor` Defender))
  ;[1 1 1 1 14] If the attacker kills the defender
  (if (>= (`local.AttackerStrength`) (`local.DefenderArmor`))
    ;[1 1 1 1 14] If the defender fights AND kills the attacker
    (if (and (>= (`local.DefenderStrength`) (`local.AttackerArmor`)) DefenderFights)
      ;[1 1 1 1 14] Attacker kills defender and defender kills attacker
      (return "E_AttackerDiesDefenderDies" false)
      (else
        ;[1 1 1 1 14] Attacker kills defender and attacker survives
        (return "E_AttackerSurvivesDefenderDies" false)))
    (elif DefenderFights
      ;[1 1 1 1 14] If the defender kills the attacker
      (if (>= (`local.DefenderStrength`) (`local.AttackerArmor`))
        ;[1 1 1 1 14] Defender survives, defender kills attacker
        (return "E_DefenderSurvivesAttackerDies" false)
        (else
          ;[1 1 1 1 14] Defender survives, attacker survives: deadlock
          (return "E_AttackerSurvivesDefenderSurvives" false)))
      (else
        ;[1 1 1 1 14] Defender survives, defender doesn't fight back
        (return "E_DefenderSurvives" false)))))

(fn `ResetInto360`
  (params (NumberToReset :type "Float (double-precision)"))
  (returns (ResetNumber :type "Float (double-precision)"))
  (if (>= NumberToReset 360.0)
    (return (- NumberToReset (`KismetMathLibrary.Conv_IntToDouble` (* (`KismetMathLibrary.FTrunc` (/ NumberToReset 360.0)) 360))))
    (elif (<= NumberToReset 0.0)
      (return NumberToReset))))

(fn `UserConstructionScript`)