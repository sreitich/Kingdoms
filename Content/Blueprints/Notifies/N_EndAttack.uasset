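; Anim notify that marks the end of an attack animation in the match and advances the attack sequence once both pieces have finished.
; It clears Attacking on the BaseAnimBP, then on the server uses a FirstAttackAnimFinished flag in the match game state as a two-piece barrier.
; The second notify resets PiecesAnimated and calls ServerAnimateAttackOutcome on the owner's instigating player pawn.
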(fn `Received_Notify`
  (params (MeshComp :type "SkeletalMeshComponent Object Reference") (Animation :type "AnimSequenceBase Object Reference"))
  (returns (ReturnValue :type Boolean))
  (bind _returnvalue (`ActorComponent.GetOwner` MeshComp))
  ;[1 1 1] Trigger the end of the attack animation call the next segment of the attack sequence when both pieces finish their animations.
  (bind _asbase_anim_bp (cast `/Game/Animations/Parent/BaseAnimBP` (`SkeletalMeshComponent.GetAnimInstance` MeshComp)))
  (set `AnimInstance_Parent.bAttacking` false _asbase_anim_bp)
  (bind _asbp_match_game_state_base (cast `/Game/Blueprints/Framework/Match/BP_Match_GameStateBase` (`GameplayStatics.GetGameState`)))
  (if (`Actor.HasAuthority` _returnvalue)
    (if (`/Game/Blueprints/Framework/Match/BP_Match_GameStateBase.FirstAttackAnimFinished` _asbp_match_game_state_base)
      (bind _asbp_match_player_pawn (cast `/Game/Blueprints/Framework/Match/BP_Match_PlayerPawn` (`Actor.Instigator` _returnvalue)))
      (set `/Game/Blueprints/Framework/Match/BP_Match_GameStateBase.PiecesAnimated` false _asbp_match_game_state_base)
      (`/Game/Blueprints/Framework/Match/BP_Match_PlayerPawn.Server_AnimateAttackOutcome` _asbp_match_player_pawn)
      (else
        (set `/Game/Blueprints/Framework/Match/BP_Match_GameStateBase.FirstAttackAnimFinished` true _asbp_match_game_state_base))))
  (return false))