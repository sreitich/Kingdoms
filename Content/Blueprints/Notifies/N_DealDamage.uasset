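; Anim notify that triggers damage reactions and effects when an animation reaches its hit moment during an attack between pieces.
; If the defender in the GameState's current attack info does not fight back, it flags the defender's anim instance to play a taking-damage animation.
; On the server only, it has the owning piece's instigator pawn multicast the damage effects, passing whether that piece is the attacker.
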(fn `Received_Notify`
  (params (MeshComp :type "SkeletalMeshComponent Object Reference") (Animation :type "AnimSequenceBase Object Reference"))
  (returns (ReturnValue :type Boolean))
  (bind _returnvalue (`ActorComponent.GetOwner` MeshComp))
  ;[1 1 1] If the defender doesn't fight back, it plays a "taking damage" animation.
  (bind _asbp_match_game_state_base (cast `/Game/Blueprints/Framework/Match/BP_Match_GameStateBase` (`GameplayStatics.GetGameState`)))
  (bind (_currentattackinfo_attacker _currentattackinfo_defender _currentattackinfo_bmoveto _currentattackinfo_bmoved _currentattackinfo_bdefenderfights) (break `AttackInfo` (`/Game/Blueprints/Framework/Match/BP_Match_GameStateBase.CurrentAttackInfo` _asbp_match_game_state_base)))
  (if (not _currentattackinfo_bdefenderfights)
    (bind _asbase_anim_bp (cast `/Game/Animations/Parent/BaseAnimBP` (`SkeletalMeshComponent.GetAnimInstance` (`Character.Mesh` _currentattackinfo_defender))))
    (set `AnimInstance_Parent.bTakingDamage` true _asbase_anim_bp))
  ;[1 1 1 1 14] Only call this on the server.
  (if (`Actor.HasAuthority` _returnvalue)
    ;[1 1 1 1 14] Determine whether this piece is the attacker to decide which piece to spawn the damage effects on.
    (bind _asbp_match_game_state_base_2 (cast `/Game/Blueprints/Framework/Match/BP_Match_GameStateBase` (`GameplayStatics.GetGameState`)))
    (bind _asparent_piece (cast `ParentPiece` _returnvalue))
    ;[1 1 1 1 14] Animate the damage effects on each client using this piece's owning player's pawn.
    (bind _asbp_match_player_pawn (cast `/Game/Blueprints/Framework/Match/BP_Match_PlayerPawn` (`Actor.Instigator` _returnvalue)))
    (bind _currentattackinfo_attacker_2 (break `AttackInfo` (`/Game/Blueprints/Framework/Match/BP_Match_GameStateBase.CurrentAttackInfo` _asbp_match_game_state_base_2)))
    (`/Game/Blueprints/Framework/Match/BP_Match_PlayerPawn.Multicast_AnimateDamageEffects` _asbp_match_player_pawn (== _asparent_piece _currentattackinfo_attacker_2))
    (return true)
    (else
      (return false) ; This notify was not called on the server.
    )))