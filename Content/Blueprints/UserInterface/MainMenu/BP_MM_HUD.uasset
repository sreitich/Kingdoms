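; BP_MM_HUD is the main menu HUD, which manages invitation pop-up widgets for Steam friend invites.
; A single event either removes or creates a pop-up for a given friend, depending on a Destroy flag.
; It searches existing WBP_MM_InvitationPopUp widgets by sender, removing matches or creating a new pop-up only when that friend has none.
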(fn `UserConstructionScript`)