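; Poison shield VFX actor that plays a looping sequence of spawning smoke, winds, a glowing sphere, a ground decal and bubbles.
; BeginPlay creates dynamic materials, then runs parallel delay-staggered branches that toggle particles and visibility.
; Timelines scale the winds and decal, lerp the sphere from emissive to its normal look, and fade sphere and decal opacity.
; After about 14 seconds the effect resets and loops back to replay.
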(event `self.ReceiveBeginPlay`
  (bind _winds (`self.Winds`))
  (bind _decal (`self.Decal`))
  (bind _sphere (`self.Sphere`))
  (bind _sphere_2 (`self.Sphere`))
  (bind _decal_2 (`self.Decal`))
  ;[1 1 1] Begin Play
  ;[1 1 1] Create dynamic materials
  (bind _returnvalue (`PrimitiveComponent.CreateDynamicMaterialInstance` _decal 0 (`PrimitiveComponent.GetMaterial` _decal 0) "None"))
  (set `self.DecalMaterial` _returnvalue)
  (bind _returnvalue_2 (`PrimitiveComponent.CreateDynamicMaterialInstance` _sphere 0 (`PrimitiveComponent.GetMaterial` _sphere 0) "None"))
  (set `self.SphereMaterial` _returnvalue_2)
  (`KismetSystemLibrary.Delay` 1.0 :!label _label)
  (`ActorComponent.SetActive` (`self.P_Poison_SpawningSmoke`) true false)
  (`KismetSystemLibrary.Delay` 0.2)
  (`|ExecutionSequence`
    (:`then_0`
      ;[1 1 1] Activate particles
      (`ActorComponent.SetActive` (`self.Winds`) true false)
      (`ActorComponent.SetActive` (`self.WindPlanes`) true false)
      ;[1 1 1] Particle lifetime
      (`KismetSystemLibrary.Delay` 14.0)
      ;[1 1 1] Reset
      (`ActorComponent.SetActive` (`self.Winds`) false false)
      (`ActorComponent.SetActive` (`self.WindPlanes`) false false)
      (`ActorComponent.SetActive` (`self.P_Poison_SpawningSmoke`) false false)
      (`SceneComponent.SetWorldScale3D` _winds (1.0 1.0 1.0))
      (`SceneComponent.SetVisibility` (`self.Sphere`) false false)
      (`SceneComponent.SetVisibility` (`self.Decal`) false false)
      (`ActorComponent.SetActive` (`self.Bubbles`) false false)
      (goto _label))
    (:`then_1`
      ;[1 1 1] upward fade out
      (`KismetSystemLibrary.Delay` 1.7)
      (`|ExecutionSequence`
        (:`then_0`
          (bind (_direction _newtrack_0) (`Timeline|UpwardFadeOut` :!via `PlayFromStart`)
            (:`Update`
              (`SceneComponent.SetWorldScale3D` _winds (`KismetMathLibrary.MakeVector` 1.0 1.0 _newtrack_0)))))
        (:`then_1`
          ;[1 1 1] Scale larger decal
          (`SceneComponent.SetVisibility` _decal_2 true false)
          (`|ExecutionSequence`
            (:`then_0`
              (`MaterialInstanceDynamic.SetScalarParameterValue` (`self.DecalMaterial`) "Opacity" 0.0)
              (bind (_direction_2 _newtrack_0_2) (`Timeline|Animate Decal` :!via `PlayFromStart`)
                (:`Update`
                  (`SceneComponent.SetWorldScale3D` _decal_2 (`KismetMathLibrary.MakeVector` _newtrack_0_2 _newtrack_0_2 _newtrack_0_2)))
                (:`Finished`
                  (`ActorComponent.SetActive` (`self.Bubbles`) true false))))
            (:`then_1`
              ;[1 1 1] dissolve decal
              (`KismetSystemLibrary.Delay` 6.0)
              (`MaterialInstanceDynamic.SetScalarParameterValue` (`self.SphereMaterial`) "Opacity" 0.7)
              (`|ExecutionSequence`
                (:`then_0`
                  (`KismetSystemLibrary.Delay` 2.0)
                  (`|ExecutionSequence`
                    (:`then_0`
                      (bind (_direction_3 _newtrack_1) (`Timeline|Dissolve Decal` :!via `PlayFromStart`)
                        (:`Update`
                          (`MaterialInstanceDynamic.SetScalarParameterValue` (`self.DecalMaterial`) "Opacity" _newtrack_1))))
                    (:`then_1`
                      (`KismetSystemLibrary.Delay` 1.0)
                      (`ActorComponent.SetActive` (`self.Bubbles`) false false))))
                (:`then_1`
                  (bind (_direction_4 _newtrack_1_2) (`Timeline|Fade out poisonBall` :!via `PlayFromStart`)
                    (:`Update`
                      (`MaterialInstanceDynamic.SetScalarParameterValue` (`self.SphereMaterial`) "Opacity" _newtrack_1_2))))))))))
    (:`then_2`
      ;[1 1 1] Lerp from emissive shield sphere to normal material
      (bind _returnvalue_3 (`PrimitiveComponent.CreateDynamicMaterialInstance` _sphere_2 0 (`PrimitiveComponent.GetMaterial` _sphere_2 0) "None"))
      (`MaterialInstanceDynamic.SetScalarParameterValue` _returnvalue_3 "Opacity" 0.0)
      (`KismetSystemLibrary.Delay` 1.4)
      (`SceneComponent.SetVisibility` (`self.Sphere`) true false)
      (`|ExecutionSequence`
        (:`then_0`
          (`MaterialInstanceDynamic.SetScalarParameterValue` _returnvalue_3 "Opacity" 0.7))
        (:`then_1`
          (bind (_direction_5 _newtrack_0_3) (`Timeline|EmissiveLerp` :!via `PlayFromStart`)
            (:`Update`
              (`MaterialInstanceDynamic.SetScalarParameterValue` _returnvalue_3 "EmissiveLerp" _newtrack_0_3))))))
    (:`then_3`
      ;[1 1 1] Scale wind sideways
      (bind (_direction_6 _newtrack_0_4) (`Timeline|Scale Wind Mesh` :!via `PlayFromStart`)
        (:`Update`
          (`SceneComponent.SetWorldScale3D` (`self.Scene`) (`KismetMathLibrary.MakeVector` _newtrack_0_4 _newtrack_0_4 1.0)))))))

(fn `UserConstructionScript`)