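; BP_Splash_Spawn is an effect emitter that fires volleys of five BP_Splash_Projectile actors while IsActive is set.
; A DoOnce gate on Tick starts each delayed volley and is reset to repeat it after a pause.
; Staggered Sequence branches rotate and briefly pulse the PSplashSpawn effect, spawning each projectile at the central Arrow's location with the rotation of one of five numbered arrows.
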(event `self.ReceiveBeginPlay`)

(event `self.ReceiveTick`
  (params (DeltaSeconds :type "Float (single-precision)"))
  (bind _returnvalue (`SceneComponent.K2_GetComponentRotation` (`self.Arrow4`)))
  (bind _returnvalue_2 (`SceneComponent.K2_GetComponentRotation` (`self.Arrow5`)))
  (bind _returnvalue_3 (`SceneComponent.K2_GetComponentRotation` (`self.Arrow1`)))
  (bind _returnvalue_4 (`SceneComponent.K2_GetComponentRotation` (`self.Arrow2`)))
  (bind _returnvalue_5 (`SceneComponent.K2_GetComponentRotation` (`self.Arrow3`)))
  (if (`self.IsActive`) :!label _label
    (`/Engine/EditorBlueprintResources/StandardMacros.DoOnce` false :!label _label_2
      (:`Completed`
        (`KismetSystemLibrary.Delay` 1.0)
        (`|ExecutionSequence`
          (:`then_0`
            (`SceneComponent.K2_SetWorldRotation` (`self.P_Splash_Spawn`) _returnvalue_3 false false)
            (`ActorComponent.SetActive` (`self.P_Splash_Spawn`) true false)
            (`|SpawnActorFromClass` "/Game/Assets/FantasyFX/Blueprints/BP_Splash_Projectile.BP_Splash_Projectile_C" (`KismetMathLibrary.MakeTransform` (`SceneComponent.K2_GetComponentLocation` (`self.Arrow`)) _returnvalue_3) "AlwaysSpawn" "OverrideRootScale" null null)
            (`KismetSystemLibrary.Delay` 0.1)
            (`ActorComponent.SetActive` (`self.P_Splash_Spawn`) false false)
            (`KismetSystemLibrary.Delay` 3.0))
          (:`then_1`
            (`KismetSystemLibrary.Delay` 0.1)
            (`SceneComponent.K2_SetWorldRotation` (`self.P_Splash_Spawn`) _returnvalue_4 false false)
            (`ActorComponent.SetActive` (`self.P_Splash_Spawn`) true false)
            (`|SpawnActorFromClass` "/Game/Assets/FantasyFX/Blueprints/BP_Splash_Projectile.BP_Splash_Projectile_C" (`KismetMathLibrary.MakeTransform` (`SceneComponent.K2_GetComponentLocation` (`self.Arrow`)) _returnvalue_4) "AlwaysSpawn" "OverrideRootScale" null null)
            (`KismetSystemLibrary.Delay` 0.1)
            (`ActorComponent.SetActive` (`self.P_Splash_Spawn`) false false)
            (`KismetSystemLibrary.Delay` 3.0))
          (:`then_2`
            (`KismetSystemLibrary.Delay` 0.2)
            (`SceneComponent.K2_SetWorldRotation` (`self.P_Splash_Spawn`) _returnvalue_5 false false)
            (`ActorComponent.SetActive` (`self.P_Splash_Spawn`) true false)
            (`|SpawnActorFromClass` "/Game/Assets/FantasyFX/Blueprints/BP_Splash_Projectile.BP_Splash_Projectile_C" (`KismetMathLibrary.MakeTransform` (`SceneComponent.K2_GetComponentLocation` (`self.Arrow`)) _returnvalue_5) "AlwaysSpawn" "OverrideRootScale" null null)
            (`KismetSystemLibrary.Delay` 0.1)
            (`ActorComponent.SetActive` (`self.P_Splash_Spawn`) false false)
            (`KismetSystemLibrary.Delay` 3.0))
          (:`then_3`
            (`KismetSystemLibrary.Delay` 0.3)
            (`SceneComponent.K2_SetWorldRotation` (`self.P_Splash_Spawn`) _returnvalue false false)
            (`ActorComponent.SetActive` (`self.P_Splash_Spawn`) true false)
            (`|SpawnActorFromClass` "/Game/Assets/FantasyFX/Blueprints/BP_Splash_Projectile.BP_Splash_Projectile_C" (`KismetMathLibrary.MakeTransform` (`SceneComponent.K2_GetComponentLocation` (`self.Arrow`)) _returnvalue) "AlwaysSpawn" "OverrideRootScale" null null)
            (`KismetSystemLibrary.Delay` 0.1)
            (`ActorComponent.SetActive` (`self.P_Splash_Spawn`) false false)
            (`KismetSystemLibrary.Delay` 3.0))
          (:`then_4`
            (`KismetSystemLibrary.Delay` 0.4)
            (`SceneComponent.K2_SetWorldRotation` (`self.P_Splash_Spawn`) _returnvalue_2 false false)
            (`ActorComponent.SetActive` (`self.P_Splash_Spawn`) true false)
            (`|SpawnActorFromClass` "/Game/Assets/FantasyFX/Blueprints/BP_Splash_Projectile.BP_Splash_Projectile_C" (`KismetMathLibrary.MakeTransform` (`SceneComponent.K2_GetComponentLocation` (`self.Arrow`)) _returnvalue_2) "AlwaysSpawn" "OverrideRootScale" null null)
            (`KismetSystemLibrary.Delay` 0.1)
            (`ActorComponent.SetActive` (`self.P_Splash_Spawn`) false false)
            (`KismetSystemLibrary.Delay` 3.0)
            (`|ExecutionSequence`
              (:`then_0`
                (goto _label))
              (:`then_1`
                (goto _label_2 :!via `Reset`)))))))
    (else
      (goto _label_2 :!via `Reset`))))

(fn `UserConstructionScript`)