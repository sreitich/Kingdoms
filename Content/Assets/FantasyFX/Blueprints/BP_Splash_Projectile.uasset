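; Splash projectile effect actor that plays a timed impact sequence on its first collision hit, then destroys itself.
; The hit spawns an impact particle with flipped pitch and a randomly rolled splash decal.
; Three chained timelines scale the decal, rescale the actor after a short delay, then drive the decal's Dissolve material parameter alongside the point light's intensity.
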(event `self.ReceiveBeginPlay`)

(event `self.Collision.OnComponentHit`
  (params (HitComponent :type "PrimitiveComponent Object Reference") (OtherActor :type "Actor Object Reference") (OtherComp :type "PrimitiveComponent Object Reference") (NormalImpulse :type "Vector Structure") (Hit :type "HitResult Structure (by ref)"))
  (bind (_returnvalue_roll _returnvalue_pitch _returnvalue_yaw) (`KismetMathLibrary.BreakRotator` (`self.K2_GetActorRotation`)))
  (bind (_bblockinghit _binitialoverlap _time _distance _location) (`GameplayStatics.BreakHitResult` Hit))
  (bind _returnvalue (`KismetMathLibrary.RandomFloatInRange` 0.0 360.0))
  (`/Engine/EditorBlueprintResources/StandardMacros.DoOnce` false
    (:`Completed`
      (bind _returnvalue_2 (`GameplayStatics.SpawnEmitterAtLocation` "/Game/Assets/FantasyFX/Particles/Splash/P_Splash_Impact.P_Splash_Impact" (`KismetMathLibrary.MakeVector` (+ (.x _location) 0.0) (+ (.y _location) 15.0) (.z _location)) (`KismetMathLibrary.MakeRotator` _returnvalue_roll (+ _returnvalue_pitch 180.0) _returnvalue_yaw)))
      (`SceneComponent.SetWorldScale3D` _returnvalue_2 (2.0 2.0 2.0))
      (bind _returnvalue_3 (`GameplayStatics.SpawnDecalAtLocation` "/Game/Assets/FantasyFX/Materials/Splash/M_Splash_Spawn_Impact_Decal.M_Splash_Spawn_Impact_Decal" (1.0 1.0 1.0) _location (`KismetMathLibrary.MakeRotator` _returnvalue) 5.0))
      (bind (_direction _newtrack_5) (`Timeline|Timeline_0` :!via `PlayFromStart`)
        (:`Update`
          (bind _returnvalue_4 (* _newtrack_5 2.0))
          (`SceneComponent.SetWorldScale3D` _returnvalue_3 (`KismetMathLibrary.MakeVector` _returnvalue _returnvalue_4 _returnvalue_4)))
        (:`Finished`
          (`KismetSystemLibrary.Delay` 0.2)
          (bind (_direction_2 _newtrack_6) (`Timeline|Timeline_3` :!via `PlayFromStart`)
            (:`Update`
              (`self.SetActorScale3D` (`KismetMathLibrary.MakeVector` _newtrack_6 _newtrack_6 _newtrack_6)))
            (:`Finished`
              (bind _returnvalue_5 (`DecalComponent.CreateDynamicMaterialInstance` _returnvalue_3))
              (bind (_direction_3 _newtrack_6_2 _lighttrack) (`Timeline|Timeline_4` :!via `PlayFromStart`)
                (:`Update`
                  (`MaterialInstanceDynamic.SetScalarParameterValue` _returnvalue_5 "Dissolve" _newtrack_6_2)
                  (`LightComponent.SetIntensity` (`self.PointLight`) _lighttrack))
                (:`Finished`
                  (`self.K2_DestroyActor`))))))))))

(fn `UserConstructionScript`)